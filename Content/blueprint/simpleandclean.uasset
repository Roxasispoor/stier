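; Game mode Blueprint that sets up teams and assigns joining players to them.
; On BeginPlay it spawns TeamInfos actors in a loop driven by TeamNumber and stores them in the Teams array.
; PostLogin adds each new player controller to a team's controller list, using the player count modulo TeamNumber for round-robin distribution.
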(event EventBeginPlay
  (for _index (range 0 (Variables|Default|GetTeamNumber))
    (bind _returnvalue (Game|SpawnActorfromClass "/Game/blueprint/team/TeamInfos.TeamInfos_C" (Math|Transform|MakeTransform "0, 0, 0") "Undefined" 0 0))
    (Utilities|Array|AddUnique (Variables|Default|GetTeams) _returnvalue)))

(event EventTick
  (params (DeltaSeconds :type Float%20%28single-precision%29)))

(event EventPostLogin
  (params (NewPlayer :type Player%20Controller%20Object%20Reference))
  (Utilities|Array|AddUnique (Variables|/Game/blueprint/team/TeamInfos.TeamInfos_C|GetPlayersControllers (Utilities|Array|Get(acopy) (Variables|Default|GetTeams) (Math|Integer|%(Integer) (Variables|Default|GetPlayerNumber) (Variables|Default|GetTeamNumber)))) NewPlayer)
  (Math|Integer|IncrementInt (Variables|Default|GetPlayerNumber)))

(fn ConstructionScript)