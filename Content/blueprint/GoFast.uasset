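; GoFast is an effect Blueprint that speeds up a flying_char when ApplyEffect is called on it.
; It casts the passed object to flying_char, then sets MaxAcceleration to twice GetMaxSpeed (not the previous acceleration) and doubles MaxWalkSpeed.
; Only walk speed is raised directly among the movement speeds, and nothing here reverts the change.
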(event EventBeginPlay
  (|CallParentFunction) ; This node is disabled and will not be called.\nDrag off pins to build functionality.
)

(event Collision|EventActorBeginOverlap
  (params (OtherActor :type Actor%20Object%20Reference))
  (|CallParentFunction OtherActor) ; This node is disabled and will not be called.\nDrag off pins to build functionality.
)

(event EventTick
  (params (DeltaSeconds :type Float%20%28single-precision%29))
  (|CallParentFunction DeltaSeconds) ; This node is disabled and will not be called.\nDrag off pins to build functionality.
)

(event EventApplyEffect
  (params (NewParam :type Actor%20Object%20Reference))
  (bind _asflying_char (Utilities|Casting|CastToflying_char NewParam))
  (Variables|/Script/Engine.CharacterMovementComponent|SetMaxAcceleration (Variables|/Script/Engine.Character|GetCharacterMovement _asflying_char) (* 2 (Class|MovementComponent|GetMaxSpeed (Variables|/Script/Engine.Character|GetCharacterMovement _asflying_char))))
  (Variables|/Script/Engine.CharacterMovementComponent|SetMaxWalkSpeed (Variables|/Script/Engine.Character|GetCharacterMovement _asflying_char) (* 2 (Variables|/Script/Engine.CharacterMovementComponent|GetMaxWalkSpeed (Variables|/Script/Engine.Character|GetCharacterMovement _asflying_char)))))

(fn ConstructionScript
  (|CallParentFunction))